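; Enemy character with montage-driven sword and big attacks, a widget health bar, and ragdoll death.
; BPCStats receives incoming damage as a negative stat change and is linked to the health bar on BeginPlay.
; BeginSwordTrace starts a looping timer of sphere traces that apply throttled damage until EndSwordTrace, while PointDamageTrace performs a single radius hit.
; Die disables movement, enables mesh physics and flags IsDead, blocking further sword damage.
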(event `self.ReceiveBeginPlay`
  (bind _aswb_enemy_health (cast `/Game/UI/WB_enemyHealth` (`WidgetComponent.GetWidget` (`self.Widget`))))
  (`/Game/BluePrints_souls/BPC_Stats.SethealthProgressBar` (`self.BPC_Stats`) (`/Game/UI/WB_enemyHealth.healthbar` _aswb_enemy_health))
  (`/Game/BluePrints_souls/BPC_Stats.SethealthProgressBar` (`self.BPC_Stats`) (`/Game/UI/WB_enemyHealth.healthbar` _aswb_enemy_health)))

(event `self.ReceiveAnyDamage`
  (params (Damage :type "Float (single-precision)") (DamageType :type "DamageType Object Reference") (InstigatedBy :type "Controller Object Reference") (DamageCauser :type "Actor Object Reference"))
  (`/Game/BluePrints_souls/BPC_Stats.IncreaseValue` (`self.BPC_Stats`) "NewEnumerator0" (* Damage -1.0)))

(event `/Game/BluePrints_souls/BPI_damage.EndSwordTrace`
  ;[0.05208 0 0] Sword traces enemy
  (if (`KismetSystemLibrary.K2_IsValidTimerHandle` (stale `/Game/BluePrints_souls/BPI_damage.BeginSwordTrace` _returnvalue))
    (`KismetSystemLibrary.K2_ClearAndInvalidateTimerHandle` (stale `/Game/BluePrints_souls/BPI_damage.BeginSwordTrace` _returnvalue))))

(event `/Game/BluePrints_souls/BPI_damage.BeginSwordTrace`
  ;[0.05208 0 0] Sword traces enemy
  (bind _returnvalue (`KismetSystemLibrary.K2_SetTimerDelegate` (delegate `Damage Trace`) 0.1 true)))

(event `Damage Trace`
  ;[0.05208 0 0] Sword traces enemy
  (if (not (`self.isDead?`))
    (bind _outhit (`KismetSystemLibrary.SphereTraceSingleForObjects` :`Start` (`SceneComponent.K2_GetComponentLocation` (`self.Start Sword Trace pos`)) :`End` (`SceneComponent.K2_GetComponentLocation` (`self.End Sword Trace pos`)) :`Radius` 50.0 :`ObjectTypes` (`|MakeArray` "ObjectTypeQuery3" :!type "EObjectTypeQuery Enum") :`DrawDebugType` "ForOneFrame"))
    (if true
      (`/Engine/EditorBlueprintResources/StandardMacros.DoOnce` false :!label _label
        (:`Completed`
          (`GameplayStatics.ApplyDamage` (`.HitActor` (`GameplayStatics.BreakHitResult` _outhit)) (`self.sword Damage`))
          (`KismetSystemLibrary.Delay` 0.3)
          (goto _label :!via `Reset`))))))

(event `/Game/BluePrints_souls/BPI_damage.die`
  (`CharacterMovementComponent.DisableMovement` (`self.CharacterMovement`))
  (`PrimitiveComponent.SetSimulatePhysics` (`self.Mesh`) true)
  (set `self.isDead?` true))

(event `/Game/BluePrints_souls/BPI_damage.Point Damage Trace`
  (bind _returnvalue (`SceneComponent.K2_GetComponentLocation` (`self.Point Trace Pos`)))
  (bind (_outhit _returnvalue_2) (`KismetSystemLibrary.SphereTraceSingleForObjects` :`Start` _returnvalue :`End` _returnvalue :`Radius` (`self.pointAttackRadius`) :`ObjectTypes` (`|MakeArray` "ObjectTypeQuery3" :!type "EObjectTypeQuery Enum") :`DrawDebugType` "ForDuration" :`DrawTime` 2.0))
  (if _returnvalue_2
    (`GameplayStatics.ApplyDamage` (`.HitActor` (`GameplayStatics.BreakHitResult` _outhit)) 10.0)))

(fn `BigAttack`
  (returns (Duration :type "Float (double-precision)"))
  (bind _returnvalue (`self.PlayAnimMontage` "/Game/Characters/SoulsLike/combat/BigAttack_Montage.BigAttack_Montage"))
  (return _returnvalue))

(fn `SwordAttack`
  (returns (Duration :type "Float (double-precision)"))
  (bind _returnvalue (`self.PlayAnimMontage` "/Game/Characters/SoulsLike/combat/SwordAttackCombo_Montage.SwordAttackCombo_Montage"))
  (return _returnvalue))

(fn `UserConstructionScript`)