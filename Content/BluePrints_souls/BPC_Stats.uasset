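; BPC_Stats is an actor component that holds a character's stats, currently Health clamped between zero and MaxHealth.
; IncreaseValue switches on a stat identifier, adds a signed value to Health, and triggers Die when Health reaches zero.
; Die forwards the event to the owning actor through a DieMessage call, leaving the death response to the owner.
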(event `Die`
  (message `/Game/BluePrints_souls/BPI_damage.die` (`self.GetOwner`)))

(fn `IncreaseValue`
  (params (Stat :type "/Game/BluePrints_souls/E_Stats Enum" :default "NewEnumerator0") (Value :type "Float (double-precision)"))
  (switch `/Game/BluePrints_souls/E_Stats` Stat
    (:`NewEnumerator0`
      (set `self.health` (`KismetMathLibrary.FClamp` (+ (`self.health`) Value) 0.0 (`self.maxHealth`)))
      (`|ExecutionSequence`
        (:`then_0`
          (if (<= (`self.health`) 0.0)
            (`self.Die`)))))))